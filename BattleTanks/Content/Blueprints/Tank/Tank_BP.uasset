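; Tank Blueprint that handles camera aiming and supplies its Barrel through SetBarrelReference on BeginPlay.
; PlayerYaw input rotates the CameraTurnplate while PlayerPitch input rotates the SpringArm, keeping yaw and pitch on separate components.
; Both axes add relative rotation scaled by AimSpeed, with no delta-time scaling or pitch clamp in the graph.
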(event `self.ReceiveBeginPlay`
  (`self.SetBarrelReference` (`self.Barrel`)))

(event `InputAxis|PlayerPitch`
  (params (AxisValue :type "Float (single-precision)"))
  ;[1 1 1] Controls
  (`SceneComponent.K2_AddRelativeRotation` (`self.SpringArm`) (`KismetMathLibrary.MakeRotator` 0.0 (* AxisValue (`self.AimSpeed`))) false false))

(event `InputAxis|PlayerYaw`
  (params (AxisValue :type "Float (single-precision)"))
  ;[1 1 1] Controls
  (`SceneComponent.K2_AddRelativeRotation` (`self.CameraTurnplate`) (`KismetMathLibrary.MakeRotator` 0.0 0.0 (* (`self.AimSpeed`) AxisValue)) false false))

(fn `UserConstructionScript`)